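; BP_Text_StateOfEntitlement is a VR gallery text label that appears only when the player is nearby.
; Each Tick it measures the distance from itself to player character 0.
; Inside a fixed radius it shows its TextRender and rotates it with a look-at rotation to face the player; otherwise it hides the text.
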(event `self.ReceiveTick`
  (params (DeltaSeconds :type "Float (single-precision)"))
  (bind _textrender (`self.TextRender`))
  (if (< (`KismetMathLibrary.VSize` (- (`self.K2_GetActorLocation`) (`self.K2_GetActorLocation` (`GameplayStatics.GetPlayerCharacter` 0)))) 300.0)
    (`SceneComponent.SetVisibility` _textrender true false)
    (`SceneComponent.K2_SetWorldRotation` (`self.TextRender`) (`KismetMathLibrary.FindLookAtRotation` (`self.K2_GetActorLocation`) (`self.K2_GetActorLocation` (`GameplayStatics.GetPlayerCharacter` 0))) false false)
    (else
      (`SceneComponent.SetVisibility` _textrender false false))))

(fn `UserConstructionScript`)